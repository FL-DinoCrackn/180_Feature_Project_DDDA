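; AI controller for the Cyclops enemy that runs the BT_EnemyBehavior tree and takes the AIPerception component from its BP_Cyclops pawn.
; Each Tick it copies whether the player pawn's first perception stimulus is currently sensed into the HasSeenPlayer blackboard key.
; A delayed lose-sight check sits behind a constant-true branch, so it never runs, and an older AIMoveTo chase is left disconnected.
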(event `self.ReceiveTick`
  (params (DeltaSeconds :type "Float (single-precision)"))
  ; [FeatProj.] Set the value of 'HasSeenPlayer' based on this Enemy's perception of the Player Pawn
  (bind _info (`AIPerceptionComponent.GetActorsPerception` (`self.AiPerception`) (`GameplayStatics.GetPlayerPawn` 0)))
  (if true
    (bind (_age _expirationage _strength _stimuluslocation _receiverlocation _tag _bsuccessfullysensed) (break `AIStimulus` (`|GetArrayItem` (`.LastSensedStimuli` (break `ActorPerceptionBlueprintInfo` _info)))))
    (`BlackboardComponent.SetValueAsBool` (`AIBlueprintHelperLibrary.GetBlackboard` null) "HasSeenPlayer" _bsuccessfullysensed)
    (else
      ;; [FeatProj.] Wait 2 seconds after losing sight of player - if still can't see player then stop chasing
      (`KismetSystemLibrary.Delay` 2.0)
      (if (not _bsuccessfullysensed)
        (`BlackboardComponent.SetValueAsBool` (`AIBlueprintHelperLibrary.GetBlackboard` null) "HasSeenPlayer" false)))))

(event `self.ReceiveBeginPlay`
  ; [FeatProj.] Run the Behavior Tree
  (`self.RunBehaviorTree` "/Game/Blueprint/EnemyCharacter/BT_EnemyBehavior.BT_EnemyBehavior")
  (bind _asbp_cyclops (cast `/Game/Blueprint/EnemyCharacter/BP_Cyclops` (`self.K2_GetPawn`)))
  (set `self.AiPerception` (`/Game/Blueprint/EnemyCharacter/BP_Cyclops.AIPerception` _asbp_cyclops)))

(fn `UserConstructionScript`)