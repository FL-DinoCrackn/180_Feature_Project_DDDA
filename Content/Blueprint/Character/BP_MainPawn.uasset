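; BP_MainPawn is a follower that trails the player's BP_MainCharacter, which it sets as its target on BeginPlay.
; Each tick, while at least FollowDistance away, it moves toward the target at constant MoveSpeed using VInterpToConstant, keeping its own height and turning its yaw to face the target.
; Inside that distance it stops moving and snaps its rotation to zero.
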(event `self.ReceiveBeginPlay`
  ; [FeatProj.] Set Player as Target
  (bind _asbp_main_character (cast `/Game/Blueprint/Character/BP_MainCharacter` (`GameplayStatics.GetPlayerCharacter` 0)))
  (set `self.Target` _asbp_main_character))

(event `self.ReceiveTick`
  (params (DeltaSeconds :type "Float (single-precision)"))
  (bind _returnvalue (`self.K2_GetActorLocation`))
  (bind (_returnvalue_x _returnvalue_y _returnvalue_z) (`KismetMathLibrary.BreakVector` (`self.K2_GetActorLocation`)))
  (bind _target (`self.Target`))
  (bind _returnvalue_2 (`self.K2_GetActorLocation` _target))
  (bind _returnvalue_3 (`KismetMathLibrary.VInterpTo_Constant` _returnvalue _returnvalue_2 DeltaSeconds (`self.MoveSpeed`)))
  (bind (_returnvalue_roll _returnvalue_pitch _returnvalue_yaw) (`KismetMathLibrary.BreakRotator` (`KismetMathLibrary.FindLookAtRotation` _returnvalue_3 _returnvalue_2)))
  ; [FeatProj.] Follow Target each frame, Alpha controls the % of distance it moves towards the target
  (`/Engine/EditorBlueprintResources/StandardMacros.IsValid` _target
    (:`Is Valid`
      ; [FeatProj.] Check if far away from target, only move if not close
      (if (>= (`KismetMathLibrary.Vector_Distance` _returnvalue _returnvalue_2) (`self.FollowDistance`))
        (`self.K2_SetActorLocationAndRotation` (`KismetMathLibrary.MakeVector` (.x _returnvalue_3) (.y _returnvalue_3) _returnvalue_z) (`KismetMathLibrary.MakeRotator` 0.0 0.0 _returnvalue_yaw))
        (else
          (`self.K2_SetActorRotation` (struct)))))))

(fn `UserConstructionScript`)